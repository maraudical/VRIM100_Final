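; Actor component that plays a sequence of voice lines at its owner's location when any actor overlaps the owner.
; Lines advance through a Delay loop timed to each clip's duration.
; End overlap halts the sequence after the current clip, which replays on re-entry, preceded by a return line if any line has completed.
; DialoguePlaying blocks re-triggering and stays set once the last line completes.
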(event Custom|DialogueBegin
  (params (OverlappedActor :type Actor%20Object%20Reference) (OtherActor :type Actor%20Object%20Reference))
  (bind _dialogueindex (Variables|Default|GetdialogueIndex))
  (bind _dialogueaudio (Variables|Default|GetdialogueAudio))
  (bind _dialogueindex_2 (Variables|Default|GetdialogueIndex))
  (bind _dialogueaudio_2 (Variables|Default|GetdialogueAudio))
  (bind _dialoguereturnaudio (Variables|Default|GetdialogueReturnAudio))
  (bind _returnvalue (Utilities|Array|Length _dialogueaudio_2))
  (bind _output (Utilities|Array|Get(acopy) _dialogueaudio _dialogueindex))
  (bind _returnvalue_2 (< _dialogueindex_2 _returnvalue))
  (if (Variables|Default|GetdialoguePlaying)
    (Variables|Default|SetdialogueStopped false)
    (else
      (Variables|Default|SetdialoguePlaying true)
      (Variables|Default|SetdialogueStopped false)
      (if _returnvalue_2
        (if (Variables|Default|GetdialogueStarted)
          (Audio|PlaySoundatLocation _dialoguereturnaudio (Transformation|GetActorLocation (Components|GetOwner)) "0, 0, 0" 1.0 1.0 0.0 "/Game/Audio/Settings/DefaultAttenuation.DefaultAttenuation" 0 0 0)
          (Utilities|FlowControl|Delay (Variables|/Script/Engine.SoundBase|GetDuration _dialoguereturnaudio)))
        (Audio|PlaySoundatLocation _output (Transformation|GetActorLocation (Components|GetOwner)) "0, 0, 0" 1.0 1.0 0.0 "/Game/Audio/Settings/DefaultAttenuation.DefaultAttenuation" 0 0 0 :!label _label)
        (Utilities|FlowControl|Delay (Variables|/Script/Engine.SoundBase|GetDuration _output))
        (if (Variables|Default|GetdialogueStopped)
          (Variables|Default|SetdialoguePlaying false)
          (else
            (Math|Integer|IncrementInt (Variables|Default|GetdialogueIndex)
              (:%20%20
                (Variables|Default|SetdialogueStarted true)
                (if _returnvalue_2
                  (goto _label))))))))))

(event Custom|DialogueStop
  (params (OverlappedActor :type Actor%20Object%20Reference) (OtherActor :type Actor%20Object%20Reference))
  (Variables|Default|SetdialogueStopped true))

(event EventBeginPlay
  (bind _returnvalue (Components|GetOwner))
  (Collision|BindEventtoOnActorBeginOverlap _returnvalue (delegate Custom|DialogueBegin))
  (Collision|BindEventtoOnActorEndOverlap _returnvalue (delegate Custom|DialogueStop))
  (Variables|Default|SetdialogueStarted false))